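; Grabbable VR prop for the escape room, built on an IsdkGrabbable component.
; Pointer events drive an "intensity" material parameter on the mesh for hover and grab feedback, and play a sound on select and unselect.
; Hitting an actor tagged "floor" starts a timer that teleports the prop back to its BeginPlay location and zeroes its linear velocity.
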(event `RespawnObject`
  (`PrimitiveComponent.SetPhysicsLinearVelocity` (`self.StaticMesh`) (0.0 0.0 0.0) false "None")
  (`self.K2_SetActorLocation` (stale `self.ReceiveBeginPlay` _output_get) false true))

(event `self.ReceiveBeginPlay`
  (bind _output_get (set `self.InitialLocation` (`self.K2_GetActorLocation`))))

(event `self.StaticMesh.OnComponentHit`
  (params (HitComponent :type "PrimitiveComponent Object Reference") (OtherActor :type "Actor Object Reference") (OtherComp :type "PrimitiveComponent Object Reference") (NormalImpulse :type "Vector Structure") (Hit :type "HitResult Structure (by ref)"))
  (if (`self.ActorHasTag` OtherActor "floor")
    (`KismetSystemLibrary.K2_SetTimerDelegate` (delegate `RespawnObject`) 3.0)))

(event `self.IsdkGrabbable.InteractionPointerEvent`
  (params (PointerEvent :type "IsdkInteractionPointerEvent Structure (by ref)"))
  (bind (_identifier _type) (break `IsdkInteractionPointerEvent` PointerEvent))
  ; Highlight & Grab Sound
  (if (`|EnumEquality` _type "Hover")
    (`MeshComponent.SetScalarParameterValueOnMaterials` (`self.StaticMesh`) "intensity" 2.0)
    (elif (`|EnumEquality` "Unhover" _type)
      (`MeshComponent.SetScalarParameterValueOnMaterials` (`self.StaticMesh`) "intensity" 0.0)
      (elif (`|EnumEquality` _type "Select")
        (`MeshComponent.SetScalarParameterValueOnMaterials` (`self.StaticMesh`) "intensity" 0.0)
        (`GameplayStatics.PlaySoundAtLocation` "/Game/EscapeRoom/SFX/Test.Test" (`self.K2_GetActorLocation`) (struct) 1.0 1.0 0.0 null null null null)
        (elif (`|EnumEquality` _type "Unselect")
          (`MeshComponent.SetScalarParameterValueOnMaterials` (`self.StaticMesh`) "intensity" 0.5)
          (`GameplayStatics.PlaySoundAtLocation` "/Game/EscapeRoom/SFX/Test.Test" (`self.K2_GetActorLocation`) (struct) 1.0 1.0 0.0 null null null null))))))

(fn `UserConstructionScript`)